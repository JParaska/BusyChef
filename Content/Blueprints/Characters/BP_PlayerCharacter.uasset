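; BP_PlayerCharacter is the player character, carrying a hot dog stand, grill and steamer stove as child-actor weapons.
; On BeginPlay, a sequence casts each child actor to WeaponBase and adds it to the WeaponComponent's Weapons array.
; The final sequence step asks the WeaponComponent to select the default weapon.
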(event EventBeginPlay
  (Utilities|FlowControl|Sequence
    (:then_0
      (bind _asweapon_base (Utilities|Casting|CastToWeaponBase (Variables|/Script/Engine.ChildActorComponent|GetChildActor (Variables|Default|GetHotDogStand))))
      (Utilities|Array|Add (Variables|/Script/BusyChef.WeaponComponent|GetWeapons (Variables|Default|GetWeaponComponent)) _asweapon_base))
    (:then_1
      (bind _asweapon_base_2 (Utilities|Casting|CastToWeaponBase (Variables|/Script/Engine.ChildActorComponent|GetChildActor (Variables|Default|GetGrill))))
      (Utilities|Array|Add (Variables|/Script/BusyChef.WeaponComponent|GetWeapons (Variables|Default|GetWeaponComponent)) _asweapon_base_2))
    (:then_2
      (bind _asweapon_base_3 (Utilities|Casting|CastToWeaponBase (Variables|/Script/Engine.ChildActorComponent|GetChildActor (Variables|Default|GetSteamerStove))))
      (Utilities|Array|Add (Variables|/Script/BusyChef.WeaponComponent|GetWeapons (Variables|Default|GetWeaponComponent)) _asweapon_base_3))
    (:then_3
      (Class|WeaponComponent|SelectDefaultWeapon (Variables|Default|GetWeaponComponent)))))

(fn ConstructionScript)
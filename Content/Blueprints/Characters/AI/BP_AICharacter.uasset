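; BP_AICharacter is an AI-controlled character Blueprint that relies on a StatsComponent for its health.
; On BeginPlay it initializes the component's stats.
; Every tick it prints its display name and current health percentage to the screen as debug output.
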(event EventBeginPlay
  (Class|CharacterStatsComponent|InitStats (Variables|Default|GetStatsComponent)))

(event EventTick
  (params (DeltaSeconds :type Float%20%28single-precision%29))
  (Development|PrintString (Utilities|String|Append (Utilities|GetDisplayName self) ": " (Utilities|String|ToString(Float) (* (Class|CharacterStatsComponent|GetHealthPercent (Variables|Default|GetStatsComponent)) 1e+02)) "%") true false "(R=0.000000,G=0.660000,B=1.000000,A=1.000000)" 0.0))

(fn ConstructionScript)
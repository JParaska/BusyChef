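; Melee AI character Blueprint that arms itself with a built-in weapon when play begins.
; On BeginPlay it casts the Sideboard child actor to WeaponBase and adds it to the WeaponComponent's weapon list.
; It then has the component select its default weapon, a step that still runs if the cast fails.
; The construction script only calls its parent.
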(event EventBeginPlay
  (Utilities|FlowControl|Sequence
    (:then_0
      (bind _asweapon_base (Utilities|Casting|CastToWeaponBase (Variables|/Script/Engine.ChildActorComponent|GetChildActor (Variables|Default|GetSideboard))))
      (Utilities|Array|Add (Variables|/Script/BusyChef.WeaponComponent|GetWeapons (Variables|Default|GetWeaponComponent)) _asweapon_base))
    (:then_1
      (Class|WeaponComponent|SelectDefaultWeapon (Variables|Default|GetWeaponComponent)))))

(fn ConstructionScript
  (|CallParentFunction))
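; Player controller for BusyChef that creates the game UI for the possessed character and switches input and pause state with the game context.
; On possess it shows the character in WBP_GameUI, then applies the current context; later changes arrive through a GameMode binding made at BeginPlay.
; BPContextChanged enables pawn input and unpauses for Game, while menu, pause and game over share UI-only input with a visible cursor.
; Escape calls PauseGame.
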(event Custom|OnGameContextChanged
  (params (OldContext :type EGameContext%20Enum :default "None") (NewContext :type EGameContext%20Enum :default "None"))
  (CallFunction|ContextChanged NewContext))

(event EventBeginPlay
  (EventDispatchers|BindEventtoOnGameContextChanged (Class|GameContextFunctionLibrary|GetBusyChefGameModeBase) (delegate Custom|OnGameContextChanged)))

(event EventPossess
  (params (PossessedPawn :type Pawn%20Object%20Reference))
  (|CallParentFunction PossessedPawn)
  (bind _ascharacter_base (Utilities|Casting|CastToCharacterBase PossessedPawn))
  (bind _returnvalue (UserInterface|CreateWidget "/Game/Blueprints/UI/WBP_GameUI.WBP_GameUI_C" self))
  (UserInterface|Viewport|AddtoViewport _returnvalue 0)
  (Class|UserWidgetBase|ShowCharacter _returnvalue _ascharacter_base)
  (CallFunction|ContextChanged (Class|GameContextFunctionLibrary|GetGameContext)))

(event Input|KeyboardEvents|Escape
  (params (Key :type Key%20Structure :default "None"))
  (:Pressed
    (Class|GameContextFunctionLibrary|PauseGame)))

(fn ConstructionScript)

(fn BPContextChanged
  (params (NewContext :type EGameContext%20Enum :default "None"))
  (switch Utilities|FlowControl|Switch|SwitchonEGameContext NewContext
    (:MainMenu
      ;[1 1 1] Game stops or pauses
      (Input|DisableInput (Pawn|GetControlledPawn) self :!label _label)
      (Input|SetInputModeUIOnly self 0 "DoNotLock")
      (Variables|Default|SetbShowMouseCursor true))
    (:Game
      ;[1 1 1] Game starts or resumes
      (if (Game|IsGamePaused)
        (Game|SetGamePaused false))
      (Input|EnableInput (Pawn|GetControlledPawn) self)
      (Input|SetInputModeGameOnly self)
      (Variables|Default|SetbShowMouseCursor false))
    (:Pause
      (Game|SetGamePaused true) ; Game pauses
      (goto _label))
    (:GameOver
      (goto _label))))